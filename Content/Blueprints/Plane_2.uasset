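; Plane_2 is a physics-driven plane actor flown with the mouse.
; Each tick it applies a local force to the Chassi component at an offset point, combining constant forward thrust with lift opposing local vertical velocity.
; MouseX and MouseY each add mass-independent torque in chassis space, and both axes drive the same combined roll and pitch vector.
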(event `self.ReceiveTick`
  (params (DeltaSeconds :type "Float (single-precision)"))
  (bind _chassi (`self.Chassi`))
  (bind _returnvalue (`PrimitiveComponent.GetPhysicsLinearVelocity` _chassi "None"))
  (`PrimitiveComponent.AddForceAtLocationLocal` _chassi (`KismetMathLibrary.MakeVector` 700000.0 0.0 (* (.z (`KismetMathLibrary.InverseTransformDirection` (`SceneComponent.K2_GetComponentToWorld` _chassi) _returnvalue)) -4000.0)) (10.0 0.0 3.0) "None"))

(event `InputAxisKey|MouseX`
  (params (AxisValue :type "Float (single-precision)"))
  (bind _chassi (`self.Chassi`))
  (`PrimitiveComponent.AddTorqueInDegrees` _chassi (`KismetMathLibrary.TransformDirection` (`SceneComponent.K2_GetComponentToWorld` _chassi) (`KismetMathLibrary.MakeVector` (* AxisValue -50.0) (* (stale `InputAxisKey|MouseY` AxisValue) 50.0))) "None" true))

(event `InputAxisKey|MouseY`
  (params (AxisValue :type "Float (single-precision)"))
  (bind _chassi (`self.Chassi`))
  (`PrimitiveComponent.AddTorqueInDegrees` _chassi (`KismetMathLibrary.TransformDirection` (`SceneComponent.K2_GetComponentToWorld` _chassi) (`KismetMathLibrary.MakeVector` (* (stale `InputAxisKey|MouseX` AxisValue) -50.0) (* AxisValue 50.0))) "None" true))

(fn `UserConstructionScript`)